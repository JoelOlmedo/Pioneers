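; BP_BuildSystem is a component for planet_controllerr that toggles a build mode and prototypes a placement preview.
; IA_Build flip-flops InBuildMode; switching off clears the preview mesh and resets its DoOnce.
; PreviewLoop line-traces from the owner's camera, spawns a preview-material cone once, then moves it to the hit point.
; The branch calling PreviewLoop is disconnected and Tick is empty, so the preview never runs.
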(event `self.ReceiveTick`
  (params (DeltaSeconds :type "Float (single-precision)")))

(event `self.ReceiveBeginPlay`
  (bind _asplanet_controllerr (cast `/Game/Camera/planet_controllerr` (`self.GetOwner`)))
  (set `self.PlanetBP` _asplanet_controllerr)
  (set `self.Camera` (`/Game/Camera/planet_controllerr.Camera` _asplanet_controllerr)))

(event `Preview Loop`
  (bind (_returnvalue_location _returnvalue_rotation) (`KismetMathLibrary.BreakTransform` (`SceneComponent.K2_GetComponentToWorld` (`self.Camera`))))
  (bind (_outhit _returnvalue) (`KismetSystemLibrary.LineTraceSingle` :`Start` _returnvalue_location :`End` (+ _returnvalue_location (* (`KismetMathLibrary.GetForwardVector` _returnvalue_rotation) 700.0)) :`TraceChannel` "TraceTypeQuery1" :`DrawDebugType` "ForDuration"))
  (if _returnvalue
    (`|ExecutionSequence`
      (:`then_0`
        (`/Engine/EditorBlueprintResources/StandardMacros.DoOnce` false :!label _label
          (:`Completed`
            (bind _returnvalue_2 (`|AddComponentByClass` (`self.PlanetBP`) "/Script/Engine.StaticMeshComponent" false (`self.BuildPreviewTransform`)))
            (bind _output_get (set `self.PreviewMesh` _returnvalue_2))
            (`StaticMeshComponent.SetStaticMesh` _output_get "/Game/StarterContent/Shapes/Shape_Cone.Shape_Cone")
            (`PrimitiveComponent.SetMaterial` (`self.PreviewMesh`) 0 "/Game/Building/M_BuildingPreview.M_BuildingPreview"))))
      (:`then_1`
        (bind _output_get_2 (set `self.BuildPreviewTransform` (`KismetMathLibrary.MakeTransform` (`.Location` (`GameplayStatics.BreakHitResult` _outhit)) (struct) (0.1 0.1 0.1))))
        (`SceneComponent.K2_SetWorldTransform` (`self.PreviewMesh`) _output_get_2 false false)))))

(event `ResetBuildMode`
  (goto _label :!via `Reset`))

(event `EnhancedInput|/Game/Inputs/Actions/IA_Build`
  (params (ActionValue :type Boolean) (ElapsedSeconds :type "Float (double-precision)") (TriggeredSeconds :type "Float (double-precision)") (InputAction :type "InputAction Object Reference" :default "/Game/Inputs/Actions/IA_Build.IA_Build"))
  (:`Started`
    (`/Engine/EditorBlueprintResources/StandardMacros.FlipFlop`
      (:`A`
        (set `self.inBuildMode` true)
        (`KismetSystemLibrary.PrintString` "build on"))
      (:`B`
        (set `self.inBuildMode` false)
        (`StaticMeshComponent.SetStaticMesh` (`self.PreviewMesh`) null)
        (set `self.PreviewMesh` null)
        (`self.ResetBuildMode`)
        (`KismetSystemLibrary.PrintString` "build off")))))