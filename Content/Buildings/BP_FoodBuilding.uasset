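; Food building actor that appears while the player's stored amount of one resource exceeds 20 and produces that same resource.
; On BeginPlay it rotates its main mesh toward the owning planet controller's camera.
; Tick polls the player controller to toggle visibility and, through a DoOnce, starts a repeating timeline that drives FoodProgress.
; Each finished timeline grants 2 units via ReceiveFood, looping until an index counter reaches five.
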(event `self.ReceiveBeginPlay`
  (bind _asplanet_controllerr (cast `/Game/Camera/planet_controllerr` (`self.GetOwner`)))
  (bind _camera (`/Game/Camera/planet_controllerr.Camera` _asplanet_controllerr))
  (`/Engine/EditorBlueprintResources/StandardMacros.IsValid` _camera
    (:`Is Valid`
      (`SceneComponent.K2_SetWorldRotation` (`self.MainBuilding`) (`KismetMathLibrary.FindLookAtRotation` (`SceneComponent.K2_GetComponentLocation` (`self.MainBuilding`)) (`SceneComponent.K2_GetComponentLocation` _camera)) false false))))

(event `self.ReceiveTick`
  (params (DeltaSeconds :type "Float (single-precision)"))
  (bind _returnvalue (`GameplayStatics.GetActorOfClass` "/Game/BP_Player_controller.BP_Player_controller_C"))
  (if (> (`BlueprintMapLibrary.Map_Find` (`/Game/BP_Player_controller.StoredResources` _returnvalue) "NewEnumerator0") 20)
    (`self.SetActorHiddenInGame` false)
    (`/Engine/EditorBlueprintResources/StandardMacros.DoOnce` false
      (:`Completed`
        (if (< (`self.Index`) 5) :!label _label
          (bind (_direction _getresource) (`Timeline|WitingTimeForResource` :!via `PlayFromStart` :!label _label_2)
            (:`Update`
              (`BlueprintMapLibrary.Map_Add` (`self.FoodProgress`) "NewEnumerator3" _getresource))
            (:`Finished`
              (`self.ReceiveFood` 2)
              (bind _result (`/Engine/EditorBlueprintResources/StandardMacros.IncrementInt` (`self.Index`))
                (:`  `
                  (set `self.Index` _result)
                  (goto _label)))))
          (else
            (goto _label_2 :!via `Stop`)))))
    (else
      (`self.SetActorHiddenInGame` true))))

(fn `ReceiveFood`
  (params (amount :type Integer))
  (bind _asbp_player_controller (cast `/Game/BP_Player_controller` (`GameplayStatics.GetPlayerController` 0)))
  (`/Game/BP_Player_controller.ReceiveResources` _asbp_player_controller "NewEnumerator0" amount))

(fn `UserConstructionScript`
  (`parent.UserConstructionScript`))