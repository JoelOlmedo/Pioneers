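; BP_StoneBuilding is a resource building that, once built, produces stone for the player indefinitely.
; BuildStone charges a fixed cost from the player controller's StoredResources, then runs a self-restarting Timeline that updates StoneProgress and pays out Amount through ReceiveStone each cycle.
; UpgradeBuildStone raises level and yield, charging an escalating cost without checking affordability.
; An older capped production loop and a resource-based visibility check remain unconnected.
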(event `UpgradeBuildStone`
  ;[1 1 1] UpgradeBuilding
  (bind _result (`/Engine/EditorBlueprintResources/StandardMacros.IncrementInt` (`self.BuildingLevel`))
    (:`  `
      (set `self.BuildingLevel` _result)
      (set `self.Amount` (+ (`self.Amount`) 2))
      (bind _returnvalue (`GameplayStatics.GetActorOfClass` "/Game/BP_Player_controller.BP_Player_controller_C"))
      (bind _storedresources (`/Game/BP_Player_controller.StoredResources` _returnvalue))
      (`BlueprintMapLibrary.Map_Add` _storedresources "NewEnumerator1" (- (`BlueprintMapLibrary.Map_Find` _storedresources "NewEnumerator1") (`self.UpgradeMaterials`)))
      (set `self.UpgradeMaterials` (+ (`self.UpgradeMaterials`) 20)))))

(event `self.ReceiveTick`
  (params (DeltaSeconds :type "Float (single-precision)")))

(event `BuildStone`
  ;[1 1 1] ResourceLoop Function
  (bind _result (`/Engine/EditorBlueprintResources/StandardMacros.IncrementInt` (`self.BuildingLevel`))
    (:`  `
      (set `self.BuildingLevel` _result)
      (bind _returnvalue (`GameplayStatics.GetActorOfClass` "/Game/BP_Player_controller.BP_Player_controller_C"))
      (bind _storedresources (`/Game/BP_Player_controller.StoredResources` _returnvalue))
      (`BlueprintMapLibrary.Map_Add` _storedresources "NewEnumerator1" (- (`BlueprintMapLibrary.Map_Find` _storedresources "NewEnumerator1") 20))
      (bind (_direction _getresource) (`Timeline|Timeline` :!via `PlayFromStart` :!label _label)
        (:`Update`
          (`BlueprintMapLibrary.Map_Add` (`self.StoneProgress`) "NewEnumerator0" _getresource))
        (:`Finished`
          (`self.ReceiveStone` (`self.Amount`))
          (bind _result_2 (`/Engine/EditorBlueprintResources/StandardMacros.IncrementInt` (`self.Index`))
            (:`  `
              (set `self.Index` _result_2)
              (goto _label :!via `PlayFromStart`))))))))

(fn `ReceiveStone`
  (params (amount :type Integer))
  (bind _asbp_player_controller (cast `/Game/BP_Player_controller` (`GameplayStatics.GetPlayerController` 0)))
  (`/Game/BP_Player_controller.ReceiveResources` _asbp_player_controller "NewEnumerator1" amount))

(fn `UserConstructionScript`
  (`parent.UserConstructionScript`))