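; BP_MainBuilding is the main building, which the game levels up at a resource cost to raise the population.
; Its upgrade event increments the level, subtracts the same material cost from three stored resources on BP_Player_controller, adds habitants, then increases the next cost by a flat step.
; The upgrade itself does no affordability check.
; ReceiveStone forwards incoming stone to the player controller's ReceiveResources.
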(event `UpgradeMainBuilding`
  ;[1 1 1] UpgradeBuilding
  (bind _result (`/Engine/EditorBlueprintResources/StandardMacros.IncrementInt` (`self.BuildingLevel`))
    (:`  `
      (set `self.BuildingLevel` _result)
      (bind _returnvalue (`GameplayStatics.GetActorOfClass` "/Game/BP_Player_controller.BP_Player_controller_C"))
      (bind _storedresources (`/Game/BP_Player_controller.StoredResources` _returnvalue))
      (`BlueprintMapLibrary.Map_Add` _storedresources "NewEnumerator1" (- (`BlueprintMapLibrary.Map_Find` _storedresources "NewEnumerator1") (`self.UpgradeMaterials`)))
      (bind _storedresources_2 (`/Game/BP_Player_controller.StoredResources` _returnvalue))
      ;[1 1 1] ResourceLoop Function
      (`BlueprintMapLibrary.Map_Add` _storedresources_2 "NewEnumerator2" (- (`BlueprintMapLibrary.Map_Find` _storedresources_2 "NewEnumerator2") (`self.UpgradeMaterials`)))
      (bind _storedresources_3 (`/Game/BP_Player_controller.StoredResources` _returnvalue))
      (`BlueprintMapLibrary.Map_Add` _storedresources_3 "NewEnumerator0" (- (`BlueprintMapLibrary.Map_Find` _storedresources_3 "NewEnumerator0") (`self.UpgradeMaterials`)))
      (set `/Game/BP_Player_controller.TotalHabitants` (+ (`/Game/BP_Player_controller.TotalHabitants` _returnvalue) 50.0) _returnvalue)
      (set `self.UpgradeMaterials` (+ (`self.UpgradeMaterials`) 40)))))

(fn `ReceiveStone`
  (params (amount :type Integer))
  (bind _asbp_player_controller (cast `/Game/BP_Player_controller` (`GameplayStatics.GetPlayerController` 0)))
  (`/Game/BP_Player_controller.ReceiveResources` _asbp_player_controller "NewEnumerator1" amount))

(fn `UserConstructionScript`
  (`parent.UserConstructionScript`))