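; BP_Food is a clickable food resource that can be gathered three times before it is destroyed.
; Each click calls ResourceClicked, spawns a BP_GatheredEffect with a capsule mesh at the actor's location and plays a rustling bush sound.
; TimesItCanBeMined counts clicks upward despite its name, and the resource type is printed on screen as debug output.
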(event `self.ReceiveActorOnClicked`
  (params (ButtonPressed :type "Key Structure"))
  (`self.ResourceClicked`)
  (`|SpawnActorFromClass` "/Game/Resource/BP_GatheredEffect.BP_GatheredEffect_C" (`KismetMathLibrary.MakeTransform` (`self.K2_GetActorLocation`)) "Undefined" "MultiplyWithRoot" null "/Game/StarterContent/Shapes/Shape_WideCapsule.Shape_WideCapsule" null)
  (bind _result (`/Engine/EditorBlueprintResources/StandardMacros.IncrementInt` (`self.TimesItCanBeMined`))
    (:`  `
      (set `self.TimesItCanBeMined` _result)
      (`KismetSystemLibrary.PrintString` (`|GetEnumeratorNameAsString` (`self.TypeOfResource`)))
      (if (< (`self.TimesItCanBeMined`) 3)
        (`GameplayStatics.PlaySound2D` "/Game/Audio/FX/ArbustoMoviendose.ArbustoMoviendose" 1.0 1.0 0.0 null null)
        (else
          (`GameplayStatics.PlaySound2D` "/Game/Audio/FX/ArbustoMoviendose.ArbustoMoviendose" 1.0 1.0 0.0 null null)
          (`self.K2_DestroyActor`))))))

(fn `UserConstructionScript`
  (`parent.UserConstructionScript`))