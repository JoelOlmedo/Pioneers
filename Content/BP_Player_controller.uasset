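; Player controller for a resource management game, handling actor selection, stored resources, stamina and a day cycle.
; Selection keeps a single actor, clearing previous ones through BPI_SelectionEvents.
; Tick counts frames down into hours and days, growing or shrinking the population daily depending on one stored resource relative to inhabitant count.
; ReceiveResources accumulates amounts per type in a map, while ConsumeStamina deducts from a total.
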(event `AddActorSelectedToList`
  (params (SelectedActor :type "Actor Object Reference"))
  (`self.DeselectAllActors`)
  (`KismetArrayLibrary.Array_Add` (`self.SelectedActors`) SelectedActor))

(event `DeselectAllActors`
  (for _array_element (`self.SelectedActors`)
    (if (`KismetSystemLibrary.DoesImplementInterface` _array_element "/Game/Building/BPI_SelectionEvents.BPI_SelectionEvents_C")
      (message `/Game/Building/BPI_SelectionEvents.DeselectThis` _array_element)))
  (`KismetArrayLibrary.Array_Clear` (`self.SelectedActors`)))

(event `self.ReceiveBeginPlay`
  ;[1 1 1] Day system
  (set `self.HorasActuales` (`self.DuracionHoras`)))

(event `self.ReceiveTick`
  (params (DeltaSeconds :type "Float (single-precision)"))
  ;[1 1 1] Day system
  (`|ExecutionSequence`
    (:`then_0`
      (set `self.HorasActuales` (- (`self.HorasActuales`) 1.0))
      (if (== (`self.HorasActuales`) 0.0)
        (`KismetSystemLibrary.Delay` 1.0)
        (set `self.Horas` (+ (`self.Horas`) 1))
        (set `self.HorasActuales` (`self.DuracionHoras`))
        (`KismetSystemLibrary.PrintString` (`KismetStringLibrary.Conv_IntToString` (`self.Horas`)))
        (if (== (`self.Horas`) 24.0)
          (set `self.NumDia` (+ (`self.NumDia`) 1))
          (set `self.Horas` 0)
          (if (> (`BlueprintMapLibrary.Map_Find` (`self.StoredResources`) "NewEnumerator0") (* (`self.TotalHabitants`) 0.1))
            (set `self.TotalHabitants` (+ (`self.TotalHabitants`) 20.0))
            (else
              (set `self.TotalHabitants` (- (`self.TotalHabitants`) 20.0)))))))))

(fn `ConsumeStamina`
  (params (stamina :type Integer))
  (bind _output_get (set `self.TotalStamina` (- (`self.TotalStamina`) stamina)))
  (`KismetSystemLibrary.PrintString` (`KismetStringLibrary.Conv_IntToString` _output_get)))

(fn `ReceiveResources`
  (params (Type :type "/Game/Resource/E_ResourceType Enum" :default "NewEnumerator0") (Amount :type Integer))
  (`|ExecutionSequence`
    (:`then_0`
      (if (`BlueprintMapLibrary.Map_Contains` (`self.StoredResources`) Type)
        (`BlueprintMapLibrary.Map_Add` (`self.StoredResources`) (`local.Type`) (+ (`BlueprintMapLibrary.Map_Find` (`self.StoredResources`) (`local.Type`)) (`local.Amount`)))
        (else
          (`BlueprintMapLibrary.Map_Add` (`self.StoredResources`) (`local.Type`) (`local.Amount`)))))
    (:`then_1`
      (`KismetSystemLibrary.PrintString` (`KismetStringLibrary.Conv_IntToString` (`BlueprintMapLibrary.Map_Find` (`self.StoredResources`) (`local.Type`)))))))

(fn `UserConstructionScript`)